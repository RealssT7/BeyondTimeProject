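; Physics cube that responds to the game's time powers (rewind and freeze) and can be grabbed and thrown.
; Tick records its transform as it moves, then pops that stack with physics off while the game mode rewinds time.
; An overlap event replays the same stack back to the start, regardless of rewind state.
; Freezing stops simulation, and unfreezing restores momentum once through an impulse and spin derived from the last saved velocity.
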(event Custom|ThrowMontage
  ;[0.4678 1 0.8469] Time Event
  (Variables|Condition|SetInThrowed true)
  (Utilities|FlowControl|Delay 0.25)
  (Variables|Condition|SetIsGrabbed false)
  (Variables|Condition|SetInThrowed false))

(event EventBeginPlay
  (bind _staticmesh (Variables|Default|GetStaticMesh))
  ;[1 1 1] System
  (Variables|InitialValue|SetInitialLocation (Transformation|GetWorldLocation _staticmesh))
  (Variables|InitialValue|SetInitialRotaion (Transformation|GetWorldRotation _staticmesh))
  (Utilities|GetCurrentGameMode
    (:Succeed
      (Utilities|Array|Add (Variables|SavedData|GetSavedTransform) (Transformation|GetWorldTransform (Variables|Default|GetStaticMesh))))))

(event EventDuringRewindTime
  (bind (_returnvalue _savetransform _returnindex) (Utilities|CompareLastTransform))
  (bind _output (Utilities|GetLastIndexTransform))
  (bind _staticmesh (Variables|Default|GetStaticMesh))
  ;[0.4678 1 0.8469] Rewind Object Position
  (bind _isinrewind (CallFunction|IsRewinding))
  (if (or _isinrewind (Variables|Condition|GetIsOverlapped))
    (Physics|SetSimulatePhysics (Variables|Default|GetStaticMesh) false)
    (Utilities|FlowControl|Delay 0.01)
    (if (.ReturnValue (Utilities|CompareLastTransform))
      (Transformation|SetWorldTransform _staticmesh _output false false)
      (if _returnvalue
        (Utilities|Array|RemoveIndex _savetransform _returnindex))
      (else
        (Transformation|SetWorldTransform _staticmesh _output false false)
        (if (Variables|Condition|GetIsOverlapped)
          (Variables|Condition|SetIsOverlapped false)
          (Variables|TimeSetting|SetCanAffectByTime true))))))

(event EventDuringForwardTime
  ;[0.4678 1 0.8469] Rewind Object Position
)

(event EventTick
  (params (DeltaSeconds :type Float%20%28single-precision%29))
  (bind _asbpfirstpersongamemode (Variables|SavedData|GetAsBPFirstPersonGameMode))
  ;[1 1 1] Update
  (Utilities|FlowControl|Sequence
    (:then_0
      (Movement|SaveLastUpdatedVelocity))
    (:then_1
      (Movement|RemoveLateUpdatedVelocity))
    (:then_2
      (bind _isinrewind (CallFunction|IsRewinding))
      (if (not _isinrewind)
        (Utilities|CompareSaveCondition
          (:else
            (Utilities|Array|Add (Variables|SavedData|GetSavedTransform) (Transformation|GetWorldTransform (Variables|Default|GetStaticMesh)))))))
    (:then_3
      (if (Math|Boolean|ANDBoolean (Variables|/Game/FirstPerson/Blueprints/BP_FirstPersonGameMode.BP_FirstPersonGameMode_C|GetWorldControlTimeMode _asbpfirstpersongamemode) (not (Variables|/Game/FirstPerson/Blueprints/BP_FirstPersonGameMode.BP_FirstPersonGameMode_C|GetIsGameEnd _asbpfirstpersongamemode)) (not (Variables|Condition|GetIsOverlapped)))
        (Variables|TimeSetting|SetCanAffectByTime false)
        (else
          (Variables|TimeSetting|SetCanAffectByTime true)
          (CallFunction|DuringRewindTime))))
    (:then_4
      (if (Variables|Condition|GetIsOverlapped)
        (CallFunction|DuringRewindTime)))))

(event EventFreezeTime
  (bind (_returnvalue _output) (Utilities|GetLastUpdatedVelocity))
  (bind _staticmesh (Variables|Default|GetStaticMesh))
  (bind _returnvalue_2 (* _output 2.5e+02))
  ;[0.4678 1 0.8469] Time Event
  (if (or (Variables|Condition|GetIsGrabbed) (Variables|Condition|GetIsOverlapped))
    (Utilities|SetSimulatePhysic true)
    (else
      (Utilities|SetSimulatePhysic false)
      (Utilities|FlowControl|DoOnce false) ; enters at Reset
    )))

(event EventCancelFreezeTime
  (bind (_returnvalue _output) (Utilities|GetLastUpdatedVelocity))
  (bind _staticmesh (Variables|Default|GetStaticMesh))
  (bind _returnvalue_2 (* _output 2.5e+02))
  ;[0.4678 1 0.8469] Time Event
  (Utilities|SetSimulatePhysic true)
  (if _returnvalue
    (Utilities|FlowControl|DoOnce false
      (:Completed
        (Physics|AddImpulse _staticmesh _returnvalue_2 "None" false)
        (Class|PrimitiveComponent|SetAllPhysicsAngularVelocityinRadians _staticmesh (/ _returnvalue_2 5.4e+04) false)))))

(event EventDuringSlowTime
  ;[0.4678 1 0.8469] Time Event
)

(event EventCancelSlowTime
  ;[0.4678 1 0.8469] Time Event
)

(event EventOnEnterOverlapEvent
  ;[1 1 1] System
  (Variables|Condition|SetIsOverlapped true)
  (Variables|TimeSetting|SetCanAffectByTime false))

(fn ConstructionScript)

(fn SaveLastUpdatedVelocity
  (bind _savedmovedvelocity (Variables|SavedData|GetSavedMovedVelocity))
  (if (and (Utilities|Operators|NotEqual(!=) (Class|PrimitiveComponent|GetPhysicsAngularVelocityinRadians (Variables|Default|GetStaticMesh) "None") (Utilities|Array|Get(acopy) _savedmovedvelocity (Utilities|Array|LastIndex _savedmovedvelocity)) 0.01) (or (Variables|Condition|GetInThrowed) (not (Variables|Condition|GetIsGrabbed))))
    (Utilities|Array|Add (Variables|SavedData|GetSavedMovedVelocity) (Transformation|GetVelocity self))))

(fn RemoveLateUpdatedVelocity
  (bind _savedmovedvelocity (Variables|SavedData|GetSavedMovedVelocity))
  (for (_ _array_index) _savedmovedvelocity
    (if (Math|Integer|InRange(Integer) _array_index 0 (- (Utilities|Array|LastIndex _savedmovedvelocity) 1) true false)
      (Utilities|Array|RemoveIndex (Variables|SavedData|GetSavedMovedVelocity) _array_index))))

(fn IsAffect
  (return (Variables|TimeSetting|GetCanAffectByTime)))

(fn IsMove
  (bind _minthreshold (CallFunction|MoveThreshold))
  (bind _ismoved (Utilities|CalculateDistance _minthreshold)
    (:true
      (Utilities|CalculateDuration))
    (:false
      _))
  (return _ismoved))

(fn IsRewinding
  (bind _asbp_first_person_game_mode (Utilities|Casting|CastToBP_FirstPersonGameMode (Game|GetGameMode)))
  (return (Variables|/Game/FirstPerson/Blueprints/BP_FirstPersonGameMode.BP_FirstPersonGameMode_C|GetIsTimeMoveBackward _asbp_first_person_game_mode)))

(fn MoveThreshold
  (return 1.0))