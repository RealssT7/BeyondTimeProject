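; TriggerBox_Twist is a one-shot trigger volume that switches on the game mode's world-control time mode when the first-person player enters it.
; It caches BP_FirstPersonGameMode on BeginPlay.
; On box overlap by the player character, it sets WorldControlTimeMode and swaps the clock hand image on the game mode's time screen widget.
; It then destroys itself after a brief delay.
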(event OnComponentBeginOverlap(Box)
  (params (OverlappedComponent :type Primitive%20Component%20Object%20Reference) (OtherActor :type Actor%20Object%20Reference) (OtherComp :type Primitive%20Component%20Object%20Reference) (OtherBodyIndex :type Integer) (bFromSweep :type Boolean) (SweepResult :type Hit%20Result%20Structure%20%28by%20ref%29))
  (bind _as_bp_first_person_game_mode (Variables|Default|GetAs%20BP%20First%20Person%20Game%20Mode))
  ;[0.9833 0.5527 1] Overlap
  (Utilities|Casting|CastToBP_FirstPersonCharacter OtherActor)
  (Variables|/Game/FirstPerson/Blueprints/BP_FirstPersonGameMode.BP_FirstPersonGameMode_C|SetWorldControlTimeMode _as_bp_first_person_game_mode true)
  (Appearance|SetBrushfromTexture (Variables|/Game/Blueprints/Widget/TimeModeScreen.TimeModeScreen_C|GetClockHandUI (Variables|/Game/FirstPerson/Blueprints/BP_FirstPersonGameMode.BP_FirstPersonGameMode_C|GetTime%20Mode%20Screen _as_bp_first_person_game_mode)) "/Game/Material/ClockHand/ClockHand3.ClockHand3" true)
  (Utilities|FlowControl|Delay 0.2)
  (Actor|DestroyActor))

(event EventBeginPlay
  ;[0.9833 0.5527 1] Overlap
  (bind _asbp_first_person_game_mode (Utilities|Casting|CastToBP_FirstPersonGameMode (Game|GetGameMode)))
  (Variables|Default|SetAs%20BP%20First%20Person%20Game%20Mode _asbp_first_person_game_mode))

(fn ConstructionScript)