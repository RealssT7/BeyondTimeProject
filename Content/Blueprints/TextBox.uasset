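; TextBox is a trigger actor that shows a sequence of dialogue lines on screen when the first-person character overlaps its Box.
; A delayed loop macro steps through the Dialogue array at TextDuration intervals, advancing DialogueIndex to set the widget's text.
; The DialogueScreen widget is created on first use, then removed when the loop completes and the actor destroys itself.
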(event OnComponentBeginOverlap(Box)
  (params (OverlappedComponent :type Primitive%20Component%20Object%20Reference) (OtherActor :type Actor%20Object%20Reference) (OtherComp :type Primitive%20Component%20Object%20Reference) (OtherBodyIndex :type Integer) (bFromSweep :type Boolean) (SweepResult :type Hit%20Result%20Structure%20%28by%20ref%29))
  ;[0.9833 0.5527 1] Overlap
  (Utilities|Casting|CastToBP_FirstPersonCharacter OtherActor)
  (CallFunction|TextPrinter))

(event Custom|TextPrinter
  (bind _dialogueindex (Variables|Data|GetDialogueIndex))
  ;[0.9833 0.5527 1] Overlap
  (Utilities|ForLoopwithDelay 0 (- (Utilities|Array|Length (Variables|Setting|GetDialogue)) 1) (Variables|Setting|GetTextDuration)
    (:Body
      (Math|Integer|IncrementInt _dialogueindex
        (:%20%20
          (if (< _dialogueindex (Utilities|Array|Length (Variables|Setting|GetDialogue)))
            (Utilities|IsValid (Variables|Data|GetWidget)
              (:Is%20Valid
                _)
              (:Is%20Not%20Valid
                (bind _returnvalue (UserInterface|CreateWidget "/Game/Blueprints/Widget/DialogueScreen.DialogueScreen_C" (Game|GetPlayerController 0)))
                (bind _output_get (Variables|Data|SetWidget _returnvalue))
                (UserInterface|Viewport|AddtoPlayerScreen _output_get -1)))
            (Rendering|Components|TextRender|SetText (Variables|/Game/Blueprints/Widget/DialogueScreen.DialogueScreen_C|GetTextBlock (Variables|Data|GetWidget)) (Utilities|Text|ToText(String) (Utilities|Array|Get(acopy) (Variables|Setting|GetDialogue) (Variables|Data|GetDialogueIndex))))))))
    (:Completed
      (Widget|RemovefromParent (Variables|Data|GetWidget))
      (Actor|DestroyActor))))

(fn ConstructionScript)