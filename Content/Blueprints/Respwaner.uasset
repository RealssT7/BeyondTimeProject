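; Respwaner is a one-shot trigger that repositions the level's DeadZone actor according to the player's height.
; On BeginPlay it finds the DeadZone and moves it using the player pawn's Z through a MakeVector helper.
; When BP_FirstPersonCharacter enters its box, it clears that character's saved transform and velocity history, moves the DeadZone from the new height, and destroys itself.
; The helper's KillDistance offset below the player is present but marked unused.
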(event OnComponentBeginOverlap(Box)
  (params (OverlappedComponent :type Primitive%20Component%20Object%20Reference) (OtherActor :type Actor%20Object%20Reference) (OtherComp :type Primitive%20Component%20Object%20Reference) (OtherBodyIndex :type Integer) (bFromSweep :type Boolean) (SweepResult :type Hit%20Result%20Structure%20%28by%20ref%29))
  ;[0.5476 0.506 1] Overlap
  (bind _asbp_first_person_character (Utilities|Casting|CastToBP_FirstPersonCharacter OtherActor))
  (Utilities|Array|Clear (Variables|/Game/FirstPerson/Blueprints/BP_FirstPersonCharacter.BP_FirstPersonCharacter_C|GetSavedTransform _asbp_first_person_character))
  (Utilities|Array|Clear (Variables|/Game/FirstPerson/Blueprints/BP_FirstPersonCharacter.BP_FirstPersonCharacter_C|GetSavedVelocity _asbp_first_person_character))
  (Transformation|SetActorLocation (Variables|Reference|GetDeadZone) (Utilities|MakeVector (.z (Transformation|GetActorLocation OtherActor))) false false)
  (Actor|DestroyActor))

(event EventBeginPlay
  ;[1 1 1] Awake
  (bind _returnvalue (Actor|GetActorOfClass "/Game/Blueprints/DeadZone.DeadZone_C"))
  (bind _output_get (Variables|Reference|SetDeadZone _returnvalue))
  (Transformation|SetActorLocation _output_get (Utilities|MakeVector (.z (Transformation|GetActorLocation (Game|Player|GetPlayerPawn 0)))) false false))

(fn ConstructionScript)