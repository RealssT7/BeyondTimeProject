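; MomentumObject is a rotating actor whose spin responds to the game's time manipulation.
; A RotatingMovement component, pivoted on the mesh's relative location, spins at the configured axis speeds.
; Slow, forward, rewind and freeze time events rescale that spin by the game mode's GlobalTimeRate and a Path direction sign.
; Those events also flip Path when pitch leaves a fixed range, debounced by DoOnce and a delay; Tick is empty.
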(event Custom|ChangePath
  (Utilities|FlowControl|DoOnce false :!label _label
    (:Completed
      (Variables|Default|SetPath (* (Variables|Default|GetPath) -1.0))
      (Utilities|FlowControl|Delay 1.0)
      (goto _label Reset))))

(event EventBeginPlay
  ;[1 1 1] System
  (Variables|/Script/Engine.RotatingMovementComponent|SetPivotTranslation (Variables|Default|GetRotatingMovement) (Variables|/Script/Engine.SceneComponent|GetRelativeLocation (Variables|Default|GetMesh)))
  (bind _asbp_first_person_game_mode (Utilities|GetCurrentGameMode)
    (:Succeed
      (Variables|Reference|SetAsBPFirstPersonGameMode _asbp_first_person_game_mode)
      (Variables|/Script/Engine.RotatingMovementComponent|SetRotationRate (Variables|Default|GetRotatingMovement) (Math|Rotator|MakeRotator (Variables|MovementSetting|GetXRotationSpeed) (Variables|MovementSetting|GetYRotationSpeed) (Variables|MovementSetting|GetZRotationSpeed))))))

(event EventDuringRewindTime
  ;[0.4678 1 0.8469] Time Event
  (if (== (Variables|Default|GetPath) 1.0)
    (Variables|/Script/Engine.RotatingMovementComponent|SetRotationRate (Variables|Default|GetRotatingMovement) (* (Math|Rotator|MakeRotator (Variables|MovementSetting|GetXRotationSpeed) (Variables|MovementSetting|GetYRotationSpeed) (Variables|MovementSetting|GetZRotationSpeed)) (* (Variables|/Game/FirstPerson/Blueprints/BP_FirstPersonGameMode.BP_FirstPersonGameMode_C|GetGlobalTimeRate (Variables|Reference|GetAsBPFirstPersonGameMode)) (Variables|Default|GetPath))))
    (else
      (Variables|/Script/Engine.RotatingMovementComponent|SetRotationRate (Variables|Default|GetRotatingMovement) (* (Math|Rotator|MakeRotator (Variables|MovementSetting|GetXRotationSpeed) (Variables|MovementSetting|GetYRotationSpeed) (Variables|MovementSetting|GetZRotationSpeed)) (* (Variables|/Game/FirstPerson/Blueprints/BP_FirstPersonGameMode.BP_FirstPersonGameMode_C|GetGlobalTimeRate (Variables|Reference|GetAsBPFirstPersonGameMode)) (Variables|Default|GetPath))))))
  (if (not (Math|Float|InRange(Float) (.pitch (Transformation|GetActorRotation self)) -3e+01 3e+01))
    (CallFunction|ChangePath)))

(event EventDuringForwardTime
  ;[0.4678 1 0.8469] Time Event
  (if (== (Variables|Default|GetPath) 1.0)
    (Variables|/Script/Engine.RotatingMovementComponent|SetRotationRate (Variables|Default|GetRotatingMovement) (* (Math|Rotator|MakeRotator (Variables|MovementSetting|GetXRotationSpeed) (Variables|MovementSetting|GetYRotationSpeed) (Variables|MovementSetting|GetZRotationSpeed)) (* (Variables|/Game/FirstPerson/Blueprints/BP_FirstPersonGameMode.BP_FirstPersonGameMode_C|GetGlobalTimeRate (Variables|Reference|GetAsBPFirstPersonGameMode)) (Variables|Default|GetPath))))
    (else
      (Variables|/Script/Engine.RotatingMovementComponent|SetRotationRate (Variables|Default|GetRotatingMovement) (* (Math|Rotator|MakeRotator (Variables|MovementSetting|GetXRotationSpeed) (Variables|MovementSetting|GetYRotationSpeed) (Variables|MovementSetting|GetZRotationSpeed)) (* (Variables|/Game/FirstPerson/Blueprints/BP_FirstPersonGameMode.BP_FirstPersonGameMode_C|GetGlobalTimeRate (Variables|Reference|GetAsBPFirstPersonGameMode)) (Variables|Default|GetPath))))))
  (if (not (Math|Float|InRange(Float) (.pitch (Transformation|GetActorRotation self)) -3e+01 3e+01))
    (CallFunction|ChangePath)))

(event EventTick
  (params (DeltaSeconds :type Float%20%28single-precision%29))
  ;[1 1 1] System
)

(event EventFreezeTime
  ;[0.4678 1 0.8469] Time Event
  (if (== (Variables|Default|GetPath) 1.0)
    (Variables|/Script/Engine.RotatingMovementComponent|SetRotationRate (Variables|Default|GetRotatingMovement) (* (Math|Rotator|MakeRotator (Variables|MovementSetting|GetXRotationSpeed) (Variables|MovementSetting|GetYRotationSpeed) (Variables|MovementSetting|GetZRotationSpeed)) (* (Variables|/Game/FirstPerson/Blueprints/BP_FirstPersonGameMode.BP_FirstPersonGameMode_C|GetGlobalTimeRate (Variables|Reference|GetAsBPFirstPersonGameMode)) (Variables|Default|GetPath))))
    (else
      (Variables|/Script/Engine.RotatingMovementComponent|SetRotationRate (Variables|Default|GetRotatingMovement) (* (Math|Rotator|MakeRotator (Variables|MovementSetting|GetXRotationSpeed) (Variables|MovementSetting|GetYRotationSpeed) (Variables|MovementSetting|GetZRotationSpeed)) (* (Variables|/Game/FirstPerson/Blueprints/BP_FirstPersonGameMode.BP_FirstPersonGameMode_C|GetGlobalTimeRate (Variables|Reference|GetAsBPFirstPersonGameMode)) (Variables|Default|GetPath))))))
  (if (not (Math|Float|InRange(Float) (.pitch (Transformation|GetActorRotation self)) -3e+01 3e+01))
    (CallFunction|ChangePath)))

(event EventCancelFreezeTime
  ;[0.4678 1 0.8469] Time Event
  (if (== (Variables|Default|GetPath) 1.0)
    (Variables|/Script/Engine.RotatingMovementComponent|SetRotationRate (Variables|Default|GetRotatingMovement) (* (Math|Rotator|MakeRotator (Variables|MovementSetting|GetXRotationSpeed) (Variables|MovementSetting|GetYRotationSpeed) (Variables|MovementSetting|GetZRotationSpeed)) (* (Variables|/Game/FirstPerson/Blueprints/BP_FirstPersonGameMode.BP_FirstPersonGameMode_C|GetGlobalTimeRate (Variables|Reference|GetAsBPFirstPersonGameMode)) (Variables|Default|GetPath))))
    (else
      (Variables|/Script/Engine.RotatingMovementComponent|SetRotationRate (Variables|Default|GetRotatingMovement) (* (Math|Rotator|MakeRotator (Variables|MovementSetting|GetXRotationSpeed) (Variables|MovementSetting|GetYRotationSpeed) (Variables|MovementSetting|GetZRotationSpeed)) (* (Variables|/Game/FirstPerson/Blueprints/BP_FirstPersonGameMode.BP_FirstPersonGameMode_C|GetGlobalTimeRate (Variables|Reference|GetAsBPFirstPersonGameMode)) (Variables|Default|GetPath))))))
  (if (not (Math|Float|InRange(Float) (.pitch (Transformation|GetActorRotation self)) -3e+01 3e+01))
    (CallFunction|ChangePath)))

(event EventDuringSlowTime
  ;[0.4678 1 0.8469] Time Event
  (if (== (Variables|Default|GetPath) 1.0)
    (Variables|/Script/Engine.RotatingMovementComponent|SetRotationRate (Variables|Default|GetRotatingMovement) (* (Math|Rotator|MakeRotator (Variables|MovementSetting|GetXRotationSpeed) (Variables|MovementSetting|GetYRotationSpeed) (Variables|MovementSetting|GetZRotationSpeed)) (* (Variables|/Game/FirstPerson/Blueprints/BP_FirstPersonGameMode.BP_FirstPersonGameMode_C|GetGlobalTimeRate (Variables|Reference|GetAsBPFirstPersonGameMode)) (Variables|Default|GetPath))))
    (else
      (Variables|/Script/Engine.RotatingMovementComponent|SetRotationRate (Variables|Default|GetRotatingMovement) (* (Math|Rotator|MakeRotator (Variables|MovementSetting|GetXRotationSpeed) (Variables|MovementSetting|GetYRotationSpeed) (Variables|MovementSetting|GetZRotationSpeed)) (* (Variables|/Game/FirstPerson/Blueprints/BP_FirstPersonGameMode.BP_FirstPersonGameMode_C|GetGlobalTimeRate (Variables|Reference|GetAsBPFirstPersonGameMode)) (Variables|Default|GetPath))))))
  (if (not (Math|Float|InRange(Float) (.pitch (Transformation|GetActorRotation self)) -3e+01 3e+01))
    (CallFunction|ChangePath)))

(event EventCancelSlowTime
  ;[0.4678 1 0.8469] Time Event
  (if (== (Variables|Default|GetPath) 1.0)
    (Variables|/Script/Engine.RotatingMovementComponent|SetRotationRate (Variables|Default|GetRotatingMovement) (* (Math|Rotator|MakeRotator (Variables|MovementSetting|GetXRotationSpeed) (Variables|MovementSetting|GetYRotationSpeed) (Variables|MovementSetting|GetZRotationSpeed)) (* (Variables|/Game/FirstPerson/Blueprints/BP_FirstPersonGameMode.BP_FirstPersonGameMode_C|GetGlobalTimeRate (Variables|Reference|GetAsBPFirstPersonGameMode)) (Variables|Default|GetPath))))
    (else
      (Variables|/Script/Engine.RotatingMovementComponent|SetRotationRate (Variables|Default|GetRotatingMovement) (* (Math|Rotator|MakeRotator (Variables|MovementSetting|GetXRotationSpeed) (Variables|MovementSetting|GetYRotationSpeed) (Variables|MovementSetting|GetZRotationSpeed)) (* (Variables|/Game/FirstPerson/Blueprints/BP_FirstPersonGameMode.BP_FirstPersonGameMode_C|GetGlobalTimeRate (Variables|Reference|GetAsBPFirstPersonGameMode)) (Variables|Default|GetPath))))))
  (if (not (Math|Float|InRange(Float) (.pitch (Transformation|GetActorRotation self)) -3e+01 3e+01))
    (CallFunction|ChangePath)))

(fn ConstructionScript)

(fn IsAffect
  (return (Variables|TimeSetting|GetCanAffectByTime)))

(fn IsMove
  (CallFunction|MoveThreshold))

(fn IsRewinding
  (bind _asbp_first_person_game_mode (Utilities|Casting|CastToBP_FirstPersonGameMode (Game|GetGameMode)))
  (return (Variables|/Game/FirstPerson/Blueprints/BP_FirstPersonGameMode.BP_FirstPersonGameMode_C|GetIsTimeMoveBackward _asbp_first_person_game_mode)))

(fn MoveThreshold
  (return 1.0))