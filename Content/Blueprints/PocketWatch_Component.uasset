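; Pocket watch component that winds a shared global time value backward or forward.
; Two custom events cast the game mode to BP_FirstPersonGameMode and modify its GlobalTimeValue by world delta seconds on each call.
; Increment scales the step by the game mode's GlobalTimeRate, while subtract uses a fixed unit rate and ignores it.
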(event Custom|SubtractCalculation
  ;[1 1 1] Subtract
  (bind _asbp_first_person_game_mode (Utilities|Casting|CastToBP_FirstPersonGameMode (Game|GetGameMode)))
  (Variables|/Game/FirstPerson/Blueprints/BP_FirstPersonGameMode.BP_FirstPersonGameMode_C|SetGlobalTimeValue _asbp_first_person_game_mode (- (Variables|/Game/FirstPerson/Blueprints/BP_FirstPersonGameMode.BP_FirstPersonGameMode_C|GetGlobalTimeValue _asbp_first_person_game_mode) (* (Utilities|Time|GetWorldDeltaSeconds) 1.0))))

(event Custom|IncrementCalculation
  ;[1 1 1] Increment
  (bind _asbp_first_person_game_mode (Utilities|Casting|CastToBP_FirstPersonGameMode (Game|GetGameMode)))
  (Variables|/Game/FirstPerson/Blueprints/BP_FirstPersonGameMode.BP_FirstPersonGameMode_C|SetGlobalTimeValue _asbp_first_person_game_mode (+ (Variables|/Game/FirstPerson/Blueprints/BP_FirstPersonGameMode.BP_FirstPersonGameMode_C|GetGlobalTimeValue _asbp_first_person_game_mode) (* (Utilities|Time|GetWorldDeltaSeconds) (Variables|/Game/FirstPerson/Blueprints/BP_FirstPersonGameMode.BP_FirstPersonGameMode_C|GetGlobalTimeRate _asbp_first_person_game_mode)))))