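; Pocket watch Blueprint that gives time-control abilities: slow, fast-forward, freeze and rewind.
; Keys 1 and 2 toggle timelines that ease global time dilation, inversely scaling the actor's CustomTimeDilation to keep its own speed normal.
; Holding F disables DynamicCube physics, release restores it and normal time, and Q resets cube positions.
; A dilation check gates each toggle, and Tick prints global dilation for debugging.
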(event Custom|InitializeSlowWorld
  ;[1 0.7952 0.5204] Initialize Slow Time
  (Components|Timeline|SetPlayRate (Variables|Default|GetTimeline_Slow_Init) 1.5)
  (bind _duration (Timeline|Timeline_Slow_Init PlayFromStart)
    (:Update
      (Utilities|Time|SetGlobalTimeDilation (Math|Float|Lerp 1.0 0.1 _duration)))))

(event Custom|InitializeSlowCharacter
  ;[1 0.7952 0.5204] Initialize Slow Time
  (Components|Timeline|SetPlayRate (Variables|Default|GetTimeline_Slow_Pressed) 1.5)
  (bind _duration (Timeline|Timeline_Slow_Pressed PlayFromStart)
    (:Update
      (Variables|Default|SetCustomTimeDilation (Math|Float|Lerp 1.0 1e+01 _duration)))))

(event Custom|InitializeForwardCharacter
  ;[1 1 1] Initialize Forward Time
  (Components|Timeline|SetPlayRate (Variables|Default|GetTimeline_Forward_Pressed) 1.25)
  (bind _duration (Timeline|Timeline_Forward_Pressed PlayFromStart)
    (:Update
      (Variables|Default|SetCustomTimeDilation (Math|Float|Lerp 1.0 0.2 _duration)))))

(event Custom|InitializeForwardWorld
  ;[1 1 1] Initialize Forward Time
  (Components|Timeline|SetPlayRate (Variables|Default|GetTimeline_Forward_Init) 1.25)
  (bind _duration (Timeline|Timeline_Forward_Init PlayFromStart)
    (:Update
      (Utilities|Time|SetGlobalTimeDilation (Math|Float|Lerp 1.0 5.0 _duration)))))

(event Custom|StopInitializeSlow
  ;[1 0.7952 0.5204] Initialize Slow Time
  (bind _duration (Timeline|Timeline_Slow_Init ReverseFromEnd)
    (:Update
      (Utilities|Time|SetGlobalTimeDilation (Math|Float|Lerp 1.0 0.1 _duration)))))

(event Custom|StopInitializeForward
  ;[1 1 1] Initialize Forward Time
  (bind _duration (Timeline|Timeline_Forward_Init ReverseFromEnd)
    (:Update
      (Utilities|Time|SetGlobalTimeDilation (Math|Float|Lerp 1.0 5.0 _duration)))))

(event EventTick
  (params (DeltaSeconds :type Float%20%28single-precision%29))
  ;[1 0.7952 0.5204] Debug
  (Development|PrintString (Utilities|String|ToString(Float) (Class|GameplayStatics|GetGlobalTimeDilation))))

(event Input|KeyboardEvents|Q
  (params (Key :type Key%20Structure :default "None"))
  ;[0.3811 1 0.5218] Rewind Position
  (:Pressed
    (bind _outactors (Actor|GetAllActorsOfClass "/Game/Blueprints/DynamicCube.DynamicCube_C"))
    (for _array_element _outactors
      (Default|ResetPosition _array_element))))

(event Input|KeyboardEvents|2
  (params (Key :type Key%20Structure :default "None"))
  ;[1 1 1] Forward Time
  (:Pressed
    (Utilities|FlowControl|FlipFlop
      (:A
        (Utilities|IsDefaultTimeDilation 1.0
          (:true
            (bind _outactors (Actor|GetAllActorsOfClass "/Game/Blueprints/DynamicCube.DynamicCube_C"))
            (for _array_element _outactors
              (Default|IsMove _array_element))
            (CallFunction|InitializeForwardWorld)
            (CallFunction|InitializeForwardCharacter))))
      (:B
        (Utilities|IsDefaultTimeDilation 5.0
          (:true
            (Components|Timeline|SetPlayRate (Variables|Default|GetTimeline_Forward_Init) 1.5)
            (CallFunction|StopInitializeForward)
            (bind _duration (Timeline|Timeline_Forward_Released ReverseFromEnd)
              (:Update
                (Variables|Default|SetCustomTimeDilation (Math|Float|Lerp 1.0 0.2 _duration))))))))))

(event Input|KeyboardEvents|1
  (params (Key :type Key%20Structure :default "None"))
  ;[1 0.7952 0.5204] Slow Down TIme
  (:Pressed
    (Utilities|FlowControl|FlipFlop
      (:A
        (Utilities|IsDefaultTimeDilation 1.0
          (:true
            (bind _outactors (Actor|GetAllActorsOfClass "/Game/Blueprints/DynamicCube.DynamicCube_C"))
            (for _array_element _outactors
              (Default|IsMove _array_element))
            (CallFunction|InitializeSlowWorld)
            (CallFunction|InitializeSlowCharacter))))
      (:B
        (Utilities|IsDefaultTimeDilation 0.1
          (:true
            (Components|Timeline|SetPlayRate (Variables|Default|GetTimeline_Slow_Released) 2.5)
            (CallFunction|StopInitializeSlow)
            (bind _duration (Timeline|Timeline_Slow_Released ReverseFromEnd)
              (:Update
                (Variables|Default|SetCustomTimeDilation (Math|Float|Lerp 1.0 1e+01 _duration))))))))))

(event Input|KeyboardEvents|F
  (params (Key :type Key%20Structure :default "None"))
  ;[0.3811 1 0.5218] Stop Simulate Physic
  (:Pressed
    (bind _outactors (Actor|GetAllActorsOfClass "/Game/Blueprints/DynamicCube.DynamicCube_C"))
    (for _array_element _outactors
      (Physics|SetSimulatePhysics (Variables|/Game/Blueprints/DynamicCube.DynamicCube_C|GetStaticMesh _array_element) false)))
  (:Released
    (Utilities|Time|SetGlobalTimeDilation 1.0)
    (Variables|Default|SetCustomTimeDilation 1.0)
    (bind _outactors_2 (Actor|GetAllActorsOfClass "/Game/Blueprints/DynamicCube.DynamicCube_C"))
    (for _array_element_2 _outactors_2
      (Physics|SetSimulatePhysics (Variables|/Game/Blueprints/DynamicCube.DynamicCube_C|GetStaticMesh _array_element_2) true))))

(fn ConstructionScript)