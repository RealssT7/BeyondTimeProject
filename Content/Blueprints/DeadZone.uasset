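; DeadZone is a trigger volume that tells actors when they enter or leave it.
; Box overlap begin and end cast the other actor to Dead_Interface and call its enter and exit overlap events, leaving the response to that actor.
; On BeginPlay it also fetches and stores the BP_FirstPersonGameMode, which the overlap logic does not use.
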(event OnComponentBeginOverlap(Box)
  (params (OverlappedComponent :type Primitive%20Component%20Object%20Reference) (OtherActor :type Actor%20Object%20Reference) (OtherComp :type Primitive%20Component%20Object%20Reference) (OtherBodyIndex :type Integer) (bFromSweep :type Boolean) (SweepResult :type Hit%20Result%20Structure%20%28by%20ref%29))
  ;[0.9833 0.5527 1] Overlap
  (bind _asdead_interface (Utilities|Casting|CastToDead_Interface OtherActor))
  (Default|OnEnterOverlapEvent _asdead_interface))

(event OnComponentEndOverlap(Box)
  (params (OverlappedComponent :type Primitive%20Component%20Object%20Reference) (OtherActor :type Actor%20Object%20Reference) (OtherComp :type Primitive%20Component%20Object%20Reference) (OtherBodyIndex :type Integer))
  ;[0.9833 0.5527 1] Overlap
  (bind _asdead_interface (Utilities|Casting|CastToDead_Interface OtherActor))
  (Default|OnExitOverlapEvent _asdead_interface))

(event EventBeginPlay
  ;[1 1 1] Awake
  (Utilities|GetCurrentGameMode))

(fn ConstructionScript)