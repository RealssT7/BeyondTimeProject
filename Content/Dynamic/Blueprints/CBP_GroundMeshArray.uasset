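; CBP_GroundMeshArray is a Blueprint that groups twelve merged ground static mesh components so their height can be set together.
; Its SetMeshLocation event takes a MaxTop value and applies it as the relative Z location of every mesh in a single SetRelativeLocation call.
; The construction script is empty, and the event is the only logic.
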(event Custom|Set%20Mesh%20Location
  (params (Max%20Top :type Float%20%28double-precision%29))
  (Transformation|SetRelativeLocation (Variables|Default|GetSM_Ground_SM_SM_MERGED_00) (Math|Vector|MakeVector 0.0 0.0 Max%20Top) false false))

(fn ConstructionScript)