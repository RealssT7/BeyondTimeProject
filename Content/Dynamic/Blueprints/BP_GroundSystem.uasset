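; BP_GroundSystem is a ground segment actor that builds its ground pieces on demand as overlap boxes are triggered.
; The construction script spaces thirteen boxes along negative Y using the Distance array.
; Overlaps on Box through Box11 call SetGround, which spawns, attaches and animates a CBP_GroundMesh once per ID, using the matching GroundMesh entry.
; SetNewSystem can spawn a follow-on system at the last offset, but its caller and the cleanup logic are disconnected.
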(event OnComponentBeginOverlap(Box)
  (params (OverlappedComponent :type Primitive%20Component%20Object%20Reference) (OtherActor :type Actor%20Object%20Reference) (OtherComp :type Primitive%20Component%20Object%20Reference) (OtherBodyIndex :type Integer) (bFromSweep :type Boolean) (SweepResult :type Hit%20Result%20Structure%20%28by%20ref%29))
  (bind _output_get (Variables|Default|SetID 0))
  (CallFunction|SetGround _output_get OverlappedComponent))

(event OnComponentBeginOverlap(Box1)
  (params (OverlappedComponent :type Primitive%20Component%20Object%20Reference) (OtherActor :type Actor%20Object%20Reference) (OtherComp :type Primitive%20Component%20Object%20Reference) (OtherBodyIndex :type Integer) (bFromSweep :type Boolean) (SweepResult :type Hit%20Result%20Structure%20%28by%20ref%29))
  (bind _output_get (Variables|Default|SetID 1))
  (CallFunction|SetGround _output_get OverlappedComponent))

(event OnComponentBeginOverlap(Box10)
  (params (OverlappedComponent :type Primitive%20Component%20Object%20Reference) (OtherActor :type Actor%20Object%20Reference) (OtherComp :type Primitive%20Component%20Object%20Reference) (OtherBodyIndex :type Integer) (bFromSweep :type Boolean) (SweepResult :type Hit%20Result%20Structure%20%28by%20ref%29))
  (bind _output_get (Variables|Default|SetID 10))
  (CallFunction|SetGround _output_get OverlappedComponent))

(event OnComponentBeginOverlap(Box11)
  (params (OverlappedComponent :type Primitive%20Component%20Object%20Reference) (OtherActor :type Actor%20Object%20Reference) (OtherComp :type Primitive%20Component%20Object%20Reference) (OtherBodyIndex :type Integer) (bFromSweep :type Boolean) (SweepResult :type Hit%20Result%20Structure%20%28by%20ref%29))
  (bind _output_get (Variables|Default|SetID 11))
  (CallFunction|SetGround _output_get OverlappedComponent))

(event OnComponentBeginOverlap(Box2)
  (params (OverlappedComponent :type Primitive%20Component%20Object%20Reference) (OtherActor :type Actor%20Object%20Reference) (OtherComp :type Primitive%20Component%20Object%20Reference) (OtherBodyIndex :type Integer) (bFromSweep :type Boolean) (SweepResult :type Hit%20Result%20Structure%20%28by%20ref%29))
  (bind _output_get (Variables|Default|SetID 2))
  (CallFunction|SetGround _output_get OverlappedComponent))

(event OnComponentBeginOverlap(Box3)
  (params (OverlappedComponent :type Primitive%20Component%20Object%20Reference) (OtherActor :type Actor%20Object%20Reference) (OtherComp :type Primitive%20Component%20Object%20Reference) (OtherBodyIndex :type Integer) (bFromSweep :type Boolean) (SweepResult :type Hit%20Result%20Structure%20%28by%20ref%29))
  (bind _output_get (Variables|Default|SetID 3))
  (CallFunction|SetGround _output_get OverlappedComponent))

(event OnComponentBeginOverlap(Box4)
  (params (OverlappedComponent :type Primitive%20Component%20Object%20Reference) (OtherActor :type Actor%20Object%20Reference) (OtherComp :type Primitive%20Component%20Object%20Reference) (OtherBodyIndex :type Integer) (bFromSweep :type Boolean) (SweepResult :type Hit%20Result%20Structure%20%28by%20ref%29))
  (bind _output_get (Variables|Default|SetID 4))
  (CallFunction|SetGround _output_get OverlappedComponent))

(event OnComponentBeginOverlap(Box5)
  (params (OverlappedComponent :type Primitive%20Component%20Object%20Reference) (OtherActor :type Actor%20Object%20Reference) (OtherComp :type Primitive%20Component%20Object%20Reference) (OtherBodyIndex :type Integer) (bFromSweep :type Boolean) (SweepResult :type Hit%20Result%20Structure%20%28by%20ref%29))
  (bind _output_get (Variables|Default|SetID 5))
  (CallFunction|SetGround _output_get OverlappedComponent))

(event OnComponentBeginOverlap(Box6)
  (params (OverlappedComponent :type Primitive%20Component%20Object%20Reference) (OtherActor :type Actor%20Object%20Reference) (OtherComp :type Primitive%20Component%20Object%20Reference) (OtherBodyIndex :type Integer) (bFromSweep :type Boolean) (SweepResult :type Hit%20Result%20Structure%20%28by%20ref%29))
  (bind _output_get (Variables|Default|SetID 6))
  (CallFunction|SetGround _output_get OverlappedComponent))

(event OnComponentBeginOverlap(Box7)
  (params (OverlappedComponent :type Primitive%20Component%20Object%20Reference) (OtherActor :type Actor%20Object%20Reference) (OtherComp :type Primitive%20Component%20Object%20Reference) (OtherBodyIndex :type Integer) (bFromSweep :type Boolean) (SweepResult :type Hit%20Result%20Structure%20%28by%20ref%29))
  (bind _output_get (Variables|Default|SetID 7))
  (CallFunction|SetGround _output_get OverlappedComponent))

(event OnComponentBeginOverlap(Box8)
  (params (OverlappedComponent :type Primitive%20Component%20Object%20Reference) (OtherActor :type Actor%20Object%20Reference) (OtherComp :type Primitive%20Component%20Object%20Reference) (OtherBodyIndex :type Integer) (bFromSweep :type Boolean) (SweepResult :type Hit%20Result%20Structure%20%28by%20ref%29))
  (bind _output_get (Variables|Default|SetID 8))
  (CallFunction|SetGround _output_get OverlappedComponent))

(event OnComponentBeginOverlap(Box9)
  (params (OverlappedComponent :type Primitive%20Component%20Object%20Reference) (OtherActor :type Actor%20Object%20Reference) (OtherComp :type Primitive%20Component%20Object%20Reference) (OtherBodyIndex :type Integer) (bFromSweep :type Boolean) (SweepResult :type Hit%20Result%20Structure%20%28by%20ref%29))
  (bind _output_get (Variables|Default|SetID 9))
  (CallFunction|SetGround _output_get OverlappedComponent))

(event Custom|Set%20New%20System
  (bind _returnvalue (Transformation|GetActorTransform))
  (Game|SpawnActorfromClass "BP_GroundSystem_C" (Math|Transform|MakeTransform (Math|Vector|MakeVector (.x (.location _returnvalue)) (- (.y (.location _returnvalue)) (Utilities|Array|Get(acopy) (Variables|Default|GetDistance%20) 12)) (.z (.location _returnvalue))) (.rotation _returnvalue) (.scale _returnvalue)) "Undefined" "OverrideRootScale" 0 0))

(event Custom|Set%20BoxArray
  (Variables|Default|SetBox%20Array (Utilities|Array|MakeArray (Variables|Default|GetBox) (Variables|Default|GetBox1) (Variables|Default|GetBox2) (Variables|Default|GetBox3) (Variables|Default|GetBox4) (Variables|Default|GetBox5) (Variables|Default|GetBox6) (Variables|Default|GetBox7) (Variables|Default|GetBox8) (Variables|Default|GetBox9) (Variables|Default|GetBox10) (Variables|Default|GetBox11) (Variables|Default|GetBox12))))

(event Custom|Set%20Ground
  (params (ID :type Integer) (object :type Object%20Object%20Reference))
  (if (not (Utilities|Array|ContainsItem (Variables|Default|GetSetted%20ID) ID))
    (Utilities|Array|Add (Variables|Default|GetSetted%20ID) ID)
    (bind _returnvalue (Game|SpawnActorfromClass "/Game/Dynamic/Blueprints/CBP_GroundMesh.CBP_GroundMesh_C" (Math|Transform|MakeTransform "0, 0, 0" "0, 0, 0" "1.000000,1.000000,1.000000") "Undefined" "OverrideRootScale" 0 0))
    (Default|SetGroundMesh _returnvalue (Utilities|Array|Get(acopy) (Variables|Default|GetGroundMesh) ID))
    (Transformation|AttachActorToActor _returnvalue self "None" "KeepRelative" "KeepRelative" "KeepRelative" true)
    (Default|UpdateAnim _returnvalue 5e+01)
    (Utilities|Array|Add (Variables|Default|GetGround%20Actor) _returnvalue)))

(event EventBeginPlay
  (Variables|Default|SetBox%20Array (Utilities|Array|MakeArray (Variables|Default|GetBox) (Variables|Default|GetBox1) (Variables|Default|GetBox2) (Variables|Default|GetBox3) (Variables|Default|GetBox4) (Variables|Default|GetBox5) (Variables|Default|GetBox6) (Variables|Default|GetBox7) (Variables|Default|GetBox8) (Variables|Default|GetBox9) (Variables|Default|GetBox10) (Variables|Default|GetBox11) (Variables|Default|GetBox12))))

(fn ConstructionScript
  (Utilities|FlowControl|Sequence
    (:then_1
      (CallFunction|SetBoxArray)
      (for (_array_element _array_index) (Variables|Default|GetBox%20Array)
        (Transformation|SetRelativeLocation _array_element (Math|Vector|MakeVector 0.0 (* (Utilities|Array|Get(acopy) (Variables|Default|GetDistance%20) _array_index) -1.0) 2e+02) false false)))))